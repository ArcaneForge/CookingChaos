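; AI walker character that randomizes its gender, mesh, name and walk speed on BeginPlay and can be picked up by the player.
; A sphere overlap shows the name label to players and starts RotateText, a self-recalling delay loop that writes look-at pitch into the label's world Y location, not rotation.
; Interact notifies its AI_RandomWalkerController via Snatched, disables collision and attaches the walker to the player's hold point if nothing is held.
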(event `self.ReceiveBeginPlay`
  (`self.GenderSelection`))

(event `self.Sphere.OnComponentBeginOverlap`
  (params (OverlappedComponent :type "PrimitiveComponent Object Reference") (OtherActor :type "Actor Object Reference") (OtherComp :type "PrimitiveComponent Object Reference") (OtherBodyIndex :type Integer) (bFromSweep :type Boolean) (SweepResult :type "HitResult Structure (by ref)"))
  (if (`self.ActorHasTag` OtherActor "Player")
    (set `self.CharRef` OtherActor)
    (`SceneComponent.SetVisibility` (`self.Name`) true false)
    (`self.RotateText`)))

(event `self.Sphere.OnComponentEndOverlap`
  (params (OverlappedComponent :type "PrimitiveComponent Object Reference") (OtherActor :type "Actor Object Reference") (OtherComp :type "PrimitiveComponent Object Reference") (OtherBodyIndex :type Integer))
  (if (`self.ActorHasTag` OtherActor "Player")
    (`SceneComponent.SetVisibility` (`self.Name`) false false)))

(event `RotateText`
  (bind _name (`self.Name`))
  (bind (_returnvalue_roll _returnvalue_pitch) (`KismetMathLibrary.BreakRotator` (`KismetMathLibrary.FindLookAtRotation` (`self.K2_GetActorLocation`) (`self.K2_GetActorLocation` (`self.CharRef`)))))
  (if (`SceneComponent.IsVisible` _name)
    (`SceneComponent.K2_SetWorldLocation` _name (`KismetMathLibrary.MakeVector` 0.0 _returnvalue_pitch) false false)
    (`KismetSystemLibrary.Delay` 0.02)
    (`self.RotateText`)))

(fn `FemaleAICreation`
  (`self.GetAIMesh` (`self.FemaleMeshes`))
  (`self.GetRandomName` (`self.FemaleNames`)))

(fn `GenderSelection`
  (`self.RandomMovementSpeed`)
  (bind _random5050 (`self.Random5050`))
  (if (< _random5050 2)
    (`self.FemaleAICreation`)
    (else
      (`self.MaleAICreation`))))

(fn `GetAIMesh`
  (params (Array :type "Array of SkeletalMesh Object Reference"))
  (`SkinnedMeshComponent.SetSkinnedAssetAndUpdate` (`self.Mesh`) (`|GetArrayItem` Array (`KismetMathLibrary.RandomIntegerInRange` 0 (`KismetArrayLibrary.Array_Length` Array))) true))

(fn `GetRandomName`
  (params (Array :type "Array of String"))
  (`TextRenderComponent.K2_SetText` (`self.Name`) (`KismetTextLibrary.Conv_StringToText` (`|GetArrayItem` Array (`KismetMathLibrary.RandomIntegerInRange` 0 (`KismetArrayLibrary.Array_Length` Array))))))

(fn `Interact`
  (params (Interactor :type "/Game/Blueprints/Player/BP_PlayerCharacter Object Reference"))
  (returns (`Success?` :type Boolean))
  (set `self.PlayerCharacterREF` Interactor)
  (`self.PlayerPickedUpAI`)
  (return false))

(fn `MaleAICreation`
  (`self.GetAIMesh` (`self.MaleMeshes`))
  (`self.GetRandomName` (`self.MalesNames`)))

(fn `PlayerPickedUpAI`
  (bind _playercharacterref (`self.PlayerCharacterREF`))
  (bind _playercharacterref_2 (`self.PlayerCharacterREF`))
  (bind _currentiteminhand (`/Game/Blueprints/Player/BP_PlayerCharacter.CurrentItemInHand` _playercharacterref))
  (if (not (`/Game/Blueprints/Player/BP_PlayerCharacter.PlayerHoldingItem?` (`self.PlayerCharacterREF`)))
    (bind _output_get (set `/Game/Blueprints/Player/BP_PlayerCharacter.CurrentItemInHand` self (`self.PlayerCharacterREF`)))
    (bind _asai_random_walker_controller (cast `/Game/Blueprints/AI/AI_RandomWalkerController` (`AIBlueprintHelperLibrary.GetAIController` _output_get)))
    (`/Game/Blueprints/AI/AI_RandomWalkerController.Snatched!` _asai_random_walker_controller)
    (`self.K2_SetActorRotation` (`/Game/Blueprints/Player/BP_PlayerCharacter.CurrentItemInHand` (`self.PlayerCharacterREF`)) (`KismetMathLibrary.MakeRotator` 90.0 90.0 90.0) false)
    (`self.SetActorEnableCollision` _currentiteminhand false)
    (`self.K2_AttachToComponent` _currentiteminhand (`/Game/Blueprints/Player/BP_PlayerCharacter.ItemHoldLocation` _playercharacterref) "None" "SnapToTarget" "KeepRelative" "KeepRelative" true)
    (set `/Game/Blueprints/Player/BP_PlayerCharacter.PlayerHoldingItem?` true _playercharacterref_2)
    (set `/Game/Blueprints/Player/BP_PlayerCharacter.HoldingAI?` true _playercharacterref_2)))

(fn `Random5050`
  (returns (Random5050 :type Integer))
  (bind _output_get (set `self.Random5050 ` (`KismetMathLibrary.RandomIntegerInRange` 1 2)))
  (return _output_get))

(fn `RandomMovementSpeed`
  (bind _charactermovement (`self.CharacterMovement`))
  (bind _maxwalkspeed (`CharacterMovementComponent.MaxWalkSpeed` _charactermovement))
  (set `CharacterMovementComponent.MaxWalkSpeed` (`KismetMathLibrary.RandomFloatInRange` _maxwalkspeed (+ _maxwalkspeed 100.0)) _charactermovement))

(fn `UserConstructionScript`)