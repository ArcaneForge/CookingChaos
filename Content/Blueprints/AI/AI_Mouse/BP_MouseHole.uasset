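; BP_MouseHole is a spawner that releases AI mice and takes them back when they head home.
; Shortly after BeginPlay, it spawns MiceToSpawn mice, one second apart, at random points inside SpawnBox.
; A mouse flagged GoHome that enters the box is destroyed, increments MiceToSpawn, and triggers another full batch after a delay.
; ReduceSpawnNumber lowers the batch size to no less than one, while CurrentMice tracks the population.
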(event `self.ReceiveBeginPlay`
  (`KismetSystemLibrary.Delay` 6.0)
  (`self.Spawn Mouse`))

(event `Spawn Mouse`
  (bind _spawnbox (`self.SpawnBox`))
  (for _ (range 1 (+ (`self.MiceToSpawn`) 1))
    (`AIBlueprintHelperLibrary.SpawnAIFromClass` "/Game/Blueprints/AI/AI_Mouse/BP_AI_Mouse.BP_AI_Mouse_C" null (`KismetMathLibrary.RandomPointInBoundingBox` (`SceneComponent.K2_GetComponentLocation` _spawnbox) (`BoxComponent.GetScaledBoxExtent` _spawnbox)) (struct) false null)
    (`/Engine/EditorBlueprintResources/StandardMacros.IncrementInt` (`self.CurrentMice`)
      (:`  `
        (`KismetSystemLibrary.Delay` 1.0)))))

(event `self.SpawnBox.OnComponentBeginOverlap`
  (params (OverlappedComponent :type "PrimitiveComponent Object Reference") (OtherActor :type "Actor Object Reference") (OtherComp :type "PrimitiveComponent Object Reference") (OtherBodyIndex :type Integer) (bFromSweep :type Boolean) (SweepResult :type "HitResult Structure (by ref)"))
  (bind _asbp_ai_mouse (cast `/Game/Blueprints/AI/AI_Mouse/BP_AI_Mouse` OtherActor))
  (if (`/Game/Blueprints/AI/AI_Mouse/BP_AI_Mouse.GoHome?` _asbp_ai_mouse)
    (`self.K2_DestroyActor` _asbp_ai_mouse)
    (`/Engine/EditorBlueprintResources/StandardMacros.IncrementInt` (`self.MiceToSpawn`)
      (:`  `
        (`self.ReduceCurrentMice`)
        (`KismetSystemLibrary.Delay` 10.0)
        (`self.Spawn Mouse`)))))

(event `ReduceSpawnNumber`
  (if (not (<= (`self.MiceToSpawn`) 1))
    (`/Engine/EditorBlueprintResources/StandardMacros.DecrementInt` (`self.MiceToSpawn`))))

(event `ReduceCurrentMice`
  (`/Engine/EditorBlueprintResources/StandardMacros.DecrementInt` (`self.CurrentMice`)))

(fn `UserConstructionScript`)