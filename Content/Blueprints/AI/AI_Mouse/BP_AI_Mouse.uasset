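; Mouse AI that scurries away from the player and eventually heads back to a mouse hole.
; On BeginPlay it caches the player and the first BP_MouseHole found, then a looping timer with a random interval moves it to random reachable points biased away from the player.
; After 30 flee moves it returns home.
; Overlapping a tool-using player kills it, swapping to the dead mesh and decrementing the hole's spawn and mouse counts.
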(event `self.ReceiveBeginPlay`
  (bind _outactors (`GameplayStatics.GetAllActorsOfClass` "/Game/Blueprints/AI/AI_Mouse/BP_MouseHole.BP_MouseHole_C"))
  (for _array_element _outactors
    (set `self.HomeREF` _array_element)
    (break))
  (bind _asbp_player_character (cast `/Game/Blueprints/Player/BP_PlayerCharacter` (`GameplayStatics.GetPlayerCharacter` 0)))
  (set `self.PlayerREF` _asbp_player_character)
  (bind _returnvalue (`KismetSystemLibrary.K2_SetTimerDelegate` (delegate `RunAway`) (`KismetMathLibrary.RandomFloatInRange` 0.1 1.0) true))
  (set `self.TimerHandle` _returnvalue))

(event `RunAway`
  (bind _returnvalue (`self.K2_GetActorLocation`))
  (if (`self.IsDead?`)
    _
    (elif (not (`self.GoHome?`))
      (`|AIMoveTo` self (`NavigationSystemV1.K2_GetRandomReachablePointInRadius` (`KismetMathLibrary.MakeVector` (.x (+ _returnvalue (* (`KismetMathLibrary.GetForwardVector` (`KismetMathLibrary.FindLookAtRotation` _returnvalue (`self.K2_GetActorLocation` (`self.PlayerREF`)))) -200.0))) (.y (+ _returnvalue (* (`KismetMathLibrary.GetForwardVector` (`KismetMathLibrary.FindLookAtRotation` _returnvalue (`self.K2_GetActorLocation` (`self.PlayerREF`)))) -200.0))) (.z _returnvalue)) 500.0 null null) null
        (:`then`
          (`/Engine/EditorBlueprintResources/StandardMacros.IncrementInt` (`self.count`)
            (:`  `
              (if (>= (`self.count`) 30)
                (`KismetSystemLibrary.K2_ClearAndInvalidateTimerHandle` (`self.TimerHandle`))
                (set `self.GoHome?` true)
                (`self.GoHome`)))))))))

(event `self.PlayerCollision.OnComponentBeginOverlap`
  (params (OverlappedComponent :type "PrimitiveComponent Object Reference") (OtherActor :type "Actor Object Reference") (OtherComp :type "PrimitiveComponent Object Reference") (OtherBodyIndex :type Integer) (bFromSweep :type Boolean) (SweepResult :type "HitResult Structure (by ref)"))
  (bind _asbp_player_character (cast `/Game/Blueprints/Player/BP_PlayerCharacter` OtherActor))
  (if (and (`/Game/Blueprints/Player/BP_PlayerCharacter.IsUsingTool?` _asbp_player_character) (not (`self.IsDead?`)))
    (`self.Die`)
    (`MovementComponent.StopMovementImmediately` (`self.CharacterMovement`))))

(event `GoHome`
  (`|AIMoveTo` self (`self.K2_GetActorLocation` (`self.HomeREF`)) null 5.0 true))

(event `Die`
  (`SceneComponent.SetVisibility` (`self.MouseMesh`) false false)
  (`SceneComponent.SetVisibility` (`self.DeadMesh`) true false)
  (set `self.IsDead?` true)
  (`/Game/Blueprints/AI/AI_Mouse/BP_MouseHole.ReduceSpawnNumber` (`self.HomeREF`))
  (`/Game/Blueprints/AI/AI_Mouse/BP_MouseHole.ReduceCurrentMice` (`self.HomeREF`))
  (set `self.GoHome?` false))

(fn `UserConstructionScript`)