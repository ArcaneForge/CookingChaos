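; Emergency vehicle Blueprint that serves as a fire, police or ambulance unit and spawns its responder AI.
; Fire and police events swap the truck and cop meshes; the ambulance event only spawns.
; Responders appear at random points inside SpawnArea: AI_Fireman after a delay, AI_Waiter with a walk behavior tree for police and ambulance.
; EmergencyActive runs one timed red/blue light toggle sequence per call, and EmergencyEnded hides both lights.
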(event `Emergency Active`
  (`SceneComponent.ToggleVisibility` (`self.RedLight`) false)
  (`KismetSystemLibrary.Delay` 0.2)
  (`SceneComponent.ToggleVisibility` (`self.BlueLight`) false)
  (`KismetSystemLibrary.Delay` 0.5)
  (`SceneComponent.ToggleVisibility` (`self.RedLight`) false)
  (`SceneComponent.ToggleVisibility` (`self.BlueLight`) false))

(event `EmergencyEnded`
  (`SceneComponent.SetVisibility` (`self.RedLight`) false false)
  (`SceneComponent.SetVisibility` (`self.BlueLight`) false false))

(event `SpawnFireService`
  (bind _spawnarea (`self.SpawnArea`))
  ;[1 1 1] Spawn fire truck and fireman
  (`SceneComponent.SetVisibility` (`self.FireTruckMesh`) true false)
  (`SceneComponent.SetVisibility` (`self.CopMesh`) false false)
  (`KismetSystemLibrary.Delay` 3.0)
  (`AIBlueprintHelperLibrary.SpawnAIFromClass` "/Game/Blueprints/AI/AI_Fireman/AI_Fireman.AI_Fireman_C" null (`KismetMathLibrary.RandomPointInBoundingBox` (`SceneComponent.K2_GetComponentLocation` _spawnarea) (`BoxComponent.GetScaledBoxExtent` _spawnarea)) (struct) false null))

(event `SpawnPoliceService`
  (bind _spawnarea (`self.SpawnArea`))
  ;[1 1 1] Spawn police car and policeman
  (`SceneComponent.SetVisibility` (`self.FireTruckMesh`) false false)
  (`SceneComponent.SetVisibility` (`self.CopMesh`) true false)
  (`AIBlueprintHelperLibrary.SpawnAIFromClass` "/Game/Blueprints/AI/AI_Waiter.AI_Waiter_C" "/Game/Blueprints/AI/AI_Walk_BT.AI_Walk_BT" (`KismetMathLibrary.RandomPointInBoundingBox` (`SceneComponent.K2_GetComponentLocation` _spawnarea) (`BoxComponent.GetScaledBoxExtent` _spawnarea)) (struct) false null))

(event `SpawnAmbulance`
  (bind _spawnarea (`self.SpawnArea`))
  ;[1 1 1] Spawn Ambulance and medic
  (`AIBlueprintHelperLibrary.SpawnAIFromClass` "/Game/Blueprints/AI/AI_Waiter.AI_Waiter_C" "/Game/Blueprints/AI/AI_Walk_BT.AI_Walk_BT" (`KismetMathLibrary.RandomPointInBoundingBox` (`SceneComponent.K2_GetComponentLocation` _spawnarea) (`BoxComponent.GetScaledBoxExtent` _spawnarea)) (struct) false null))

(fn `UserConstructionScript`)