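; Grinder machine that turns an item carried on its moving Scene component into a BP_RefillPepperoni.
; ActivateGrinder resets Scene to Start, waits briefly, then Tick steps it along X until near End, at a largely frame-rate-dependent speed.
; On every tick near the Convert point, it destroys the first attached actor and spawns an attached refill.
; A box overlap tracks player presence in PlayerInCollision, which this graph never reads.
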(event `Activate Grinder`
  (bind _start (`self.Start`))
  (set `self.AtEnd?` false)
  (set `self.Current` _start)
  (`SceneComponent.K2_SetRelativeLocation` (`self.Scene`) _start false false)
  (`KismetSystemLibrary.Delay` 2.0)
  (set `self.ActivateGrinder?` true))

(event `self.ReceiveTick`
  (params (DeltaSeconds :type "Float (single-precision)"))
  (if (`self.ActivateGrinder?`)
    (if (not (`self.AtEnd?`))
      (set `self.Current` (+ (`self.Current`) (`KismetMathLibrary.MakeVector` (+ DeltaSeconds 2.5))))
      (if (== (`self.Current`) (`self.End`) :`ErrorTolerance` 10.0)
        (set `self.AtEnd?` true)
        (else
          (set `self.AtEnd?` false)))
      (`SceneComponent.K2_SetRelativeLocation` (`self.Scene`) (`self.Current`) false false)
      (if (== (`self.Current`) (`self.Convert`) :`ErrorTolerance` 10.0)
        (`self.K2_DestroyActor` (`|GetArrayItem` (`self.GetAttachedActors` true)))
        (bind _returnvalue (`|SpawnActorFromClass` "/Game/Blueprints/LevelAssets/BP_RefillPepperoni.BP_RefillPepperoni_C" (`SceneComponent.GetRelativeTransform` (`self.Scene`)) "Undefined" "OverrideRootScale" null null))
        (`self.K2_AttachToComponent` _returnvalue (`self.Scene`) "None" "KeepRelative" "KeepRelative" "KeepRelative" true))
      (else
        (set `self.ActivateGrinder?` false)))))

(event `self.Box.OnComponentBeginOverlap`
  (params (OverlappedComponent :type "PrimitiveComponent Object Reference") (OtherActor :type "Actor Object Reference") (OtherComp :type "PrimitiveComponent Object Reference") (OtherBodyIndex :type Integer) (bFromSweep :type Boolean) (SweepResult :type "HitResult Structure (by ref)"))
  (cast `/Game/Blueprints/Player/BP_PlayerCharacter` OtherActor)
  (set `self.PlayerInCollision?` true))

(event `self.Box.OnComponentEndOverlap`
  (params (OverlappedComponent :type "PrimitiveComponent Object Reference") (OtherActor :type "Actor Object Reference") (OtherComp :type "PrimitiveComponent Object Reference") (OtherBodyIndex :type Integer))
  (cast `/Game/Blueprints/Player/BP_PlayerCharacter` OtherActor)
  (set `self.PlayerInCollision?` false))

(fn `UserConstructionScript`)