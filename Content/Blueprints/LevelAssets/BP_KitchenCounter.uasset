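; Kitchen counter that holds one item for the player to place, pick up or combine.
; Interact routes by counter and hand state: put down (except Refill-tagged items), pick up, or call Combine on the resting BP_Ingredient with the held item.
; Items move by attaching to the counter's scene component or the player's hold point.
; When IsActive, an overlapping AI_Chef drops its item here once, without registering it as the counter's item.
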(event `CheckInteraction`
  (params (PlayerCharacter :type "/Game/Blueprints/Player/BP_PlayerCharacter Object Reference"))
  (bind _playercharacterref (`self.PlayerCharacterREF`))
  (bind _playerholdingitem_ (`/Game/Blueprints/Player/BP_PlayerCharacter.PlayerHoldingItem?` (`self.PlayerCharacterREF`)))
  (set `self.PlayerCharacterREF` PlayerCharacter)
  (if (`self.CounterHasItem?`)
    (if _playerholdingitem_
      (bind _asbp_ingredient (cast `/Game/Blueprints/LevelAssets/BP_Ingredient` (`self.ItemOnCounter`)))
      (`/Game/Blueprints/LevelAssets/BP_Ingredient.Combine` _asbp_ingredient (`/Game/Blueprints/Player/BP_PlayerCharacter.CurrentItemInHand` _playercharacterref) _playercharacterref)
      (else
        (`self.PlayerPickUpItem`)))
    (elif _playerholdingitem_
      (`self.PlayerPutDownItem`))))

(event `self.ChefCollision.OnComponentBeginOverlap`
  (params (OverlappedComponent :type "PrimitiveComponent Object Reference") (OtherActor :type "Actor Object Reference") (OtherComp :type "PrimitiveComponent Object Reference") (OtherBodyIndex :type Integer) (bFromSweep :type Boolean) (SweepResult :type "HitResult Structure (by ref)"))
  (bind _ai_chef (`self.AI_Chef`))
  (bind _asai_chef (cast `/Game/Blueprints/AI/AI_Chef/AI_Chef` OtherActor))
  (set `self.AI_Chef` _asai_chef)
  (if (`self.IsActive?`)
    (`self.K2_DetachFromActor` (`self.AI_Chef`) "KeepRelative" "KeepRelative" "KeepRelative")
    (`self.K2_AttachToComponent` (`/Game/Blueprints/AI/AI_Chef/AI_Chef.CurrentItem` (`self.AI_Chef`)) (`self.SceneComponent`) "None" "SnapToTarget" "KeepWorld" "KeepWorld" true)
    (set `/Game/Blueprints/AI/AI_Chef/AI_Chef.CurrentItem` null _ai_chef)
    (set `/Game/Blueprints/AI/AI_Chef/AI_Chef.HoldingItem?` false _ai_chef)
    (set `self.IsActive?` false)))

(fn `Interact`
  (params (Interactor :type "/Game/Blueprints/Player/BP_PlayerCharacter Object Reference"))
  (returns (`Success?` :type Boolean))
  (`self.CheckInteraction` Interactor)
  (return true))

(fn `PlayerPickUpItem`
  (bind _playercharacterref (`self.PlayerCharacterREF`))
  (`self.K2_DetachFromActor` (`self.ItemOnCounter`) "KeepWorld" "KeepWorld" "KeepWorld")
  (bind _output_get (set `/Game/Blueprints/Player/BP_PlayerCharacter.CurrentItemInHand` (`self.ItemOnCounter`) _playercharacterref))
  (`self.K2_AttachToComponent` _output_get (`/Game/Blueprints/Player/BP_PlayerCharacter.ItemHoldLocation` _playercharacterref) "None" "SnapToTarget" "KeepWorld" "KeepWorld" true)
  (set `/Game/Blueprints/Player/BP_PlayerCharacter.PlayerHoldingItem?` true (`self.PlayerCharacterREF`))
  (set `self.CounterHasItem?` false)
  (set `self.ItemOnCounter` null))

(fn `PlayerPutDownItem`
  (bind _playercharacterref (`self.PlayerCharacterREF`))
  (if (not (`self.ActorHasTag` (`/Game/Blueprints/Player/BP_PlayerCharacter.CurrentItemInHand` (`self.PlayerCharacterREF`)) "Refill"))
    (`self.K2_DetachFromActor` (`self.PlayerCharacterREF`) "KeepWorld" "KeepWorld" "KeepWorld")
    (`self.K2_AttachToComponent` (`/Game/Blueprints/Player/BP_PlayerCharacter.CurrentItemInHand` (`self.PlayerCharacterREF`)) (`self.SceneComponent`) "None" "SnapToTarget" "SnapToTarget" "KeepWorld" true)
    (set `self.ItemOnCounter` (`/Game/Blueprints/Player/BP_PlayerCharacter.CurrentItemInHand` (`self.PlayerCharacterREF`)))
    (set `self.CounterHasItem?` true)
    (set `/Game/Blueprints/Player/BP_PlayerCharacter.CurrentItemInHand` null _playercharacterref)
    (set `/Game/Blueprints/Player/BP_PlayerCharacter.PlayerHoldingItem?` false _playercharacterref)))

(fn `UserConstructionScript`
  (`parent.UserConstructionScript`))