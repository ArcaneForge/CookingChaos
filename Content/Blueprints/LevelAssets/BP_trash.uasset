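; BP_trash is a trash pickup placed in levels that the player clears by using a tool nearby.
; It caches the player character on BeginPlay, and its sphere collision overlap events track whether the player is in range.
; Tick polls the player's IsUsingTool flag while in range and destroys the actor once it is true.
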(event `self.ReceiveBeginPlay`
  (bind _asbp_player_character (cast `/Game/Blueprints/Player/BP_PlayerCharacter` (`GameplayStatics.GetPlayerCharacter` 0)))
  (set `self.PlayerCharacterREF` _asbp_player_character))

(event `self.ReceiveTick`
  (params (DeltaSeconds :type "Float (single-precision)"))
  (if (`self.PlayerInCollision?`)
    (if (`/Game/Blueprints/Player/BP_PlayerCharacter.IsUsingTool?` (`self.PlayerCharacterREF`))
      (set `self.PlayerInCollision?` false)
      (`self.K2_DestroyActor`))))

(event `self.SphereCollision.OnComponentBeginOverlap`
  (params (OverlappedComponent :type "PrimitiveComponent Object Reference") (OtherActor :type "Actor Object Reference") (OtherComp :type "PrimitiveComponent Object Reference") (OtherBodyIndex :type Integer) (bFromSweep :type Boolean) (SweepResult :type "HitResult Structure (by ref)"))
  (cast `/Game/Blueprints/Player/BP_PlayerCharacter` OtherActor)
  (set `self.PlayerInCollision?` true))

(event `self.SphereCollision.OnComponentEndOverlap`
  (params (OverlappedComponent :type "PrimitiveComponent Object Reference") (OtherActor :type "Actor Object Reference") (OtherComp :type "PrimitiveComponent Object Reference") (OtherBodyIndex :type Integer))
  (cast `/Game/Blueprints/Player/BP_PlayerCharacter` OtherActor)
  (set `self.PlayerInCollision?` false))

(fn `UserConstructionScript`)