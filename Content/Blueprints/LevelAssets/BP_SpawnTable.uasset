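; BP_SpawnTable is a level actor that tracks an ingredient stock and shows the count on a StockNumber text component.
; ReduceStock and AddStock adjust CurrentStock and refresh the text, which turns red when stock hits zero and is not recolored on restock.
; SpawnIngredient only takes one unit while stock remains, with no spawning logic here.
; Interact is a stub that returns false.
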(event `self.ReceiveBeginPlay`
  (`parent.ReceiveBeginPlay`)
  (`TextRenderComponent.K2_SetText` (`self.StockNumber`) (`KismetTextLibrary.Conv_IntToText` (`self.CurrentStock`))))

(event `ReduceStock`
  (params (AmountToReduce :type Integer))
  (bind _output_get (set `self.CurrentStock` (- (`self.CurrentStock`) AmountToReduce)))
  (`TextRenderComponent.K2_SetText` (`self.StockNumber`) (`KismetTextLibrary.Conv_IntToText` _output_get))
  (if (== (`self.CurrentStock`) 0)
    (`TextRenderComponent.SetTextRenderColor` (`self.StockNumber`) (`self.RedColour`))))

(event `AddStock`
  (params (AmountToAdd :type Integer))
  (bind _output_get (set `self.CurrentStock` (+ (`self.CurrentStock`) AmountToAdd)))
  (`TextRenderComponent.K2_SetText` (`self.StockNumber`) (`KismetTextLibrary.Conv_IntToText` _output_get)))

(fn `Interact`
  (params (Interactor :type "/Game/Blueprints/Player/BP_PlayerCharacter Object Reference"))
  (returns (`Success?` :type Boolean))
  (return false))

(fn `SpawnIngredient`
  (if (> (`self.CurrentStock`) 0)
    (`self.ReduceStock` 1)))

(fn `UserConstructionScript`
  (`parent.UserConstructionScript`))