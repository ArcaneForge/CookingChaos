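; BP_PaintSet is an interactable level actor that opens the paint menu UI.
; Its Interact function calls ShowWIdget, which lazily creates and caches WBP_PaintMenu, adds it to the viewport and makes it visible.
; It then switches the player to UI-only input and shows the mouse cursor through BP_GameplayPC.
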(event `ShowWIdget`
  (bind _returnvalue (`GameplayStatics.GetPlayerController` 0))
  (`/Engine/EditorBlueprintResources/StandardMacros.IsValid` (`self.WBP_PaintMenu`)
    (:`Is Valid`
      _)
    (:`Is Not Valid`
      (bind _returnvalue_2 (`|CreateWidget` "/Game/Blueprints/UI/MainGame/WBP_PaintMenu.WBP_PaintMenu_C" (`GameplayStatics.GetPlayerController` 0)))
      (bind _output_get (set `self.WBP_PaintMenu` _returnvalue_2))
      (`UserWidget.AddToViewport` _output_get 0)))
  (`Widget.SetVisibility` (`self.WBP_PaintMenu`) "Visible")
  (`WidgetBlueprintLibrary.SetInputMode_UIOnlyEx` _returnvalue null)
  (bind _asbp_gameplay_pc (cast `/Game/Blueprints/Player/BP_GameplayPC` _returnvalue))
  (set `PlayerController.bShowMouseCursor` true _asbp_gameplay_pc))

(fn `Interact`
  (params (Interactor :type "/Game/Blueprints/Player/BP_PlayerCharacter Object Reference"))
  (returns (`Success?` :type Boolean))
  (`self.ShowWIdget`)
  (return false))

(fn `UserConstructionScript`)