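; BP_DumpBase is a base Blueprint for trash dump level assets that display their current capacity.
; It declares AddTrash and RemoveTrash events with empty bodies, so this file contains no logic that changes the capacity.
; Each Tick writes CurrentCapacity to a text render as an integer and rotates an arrow component to face the first player character's mesh.
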(event `AddTrash`
  (params (AmountToAdd :type Integer)))

(event `RemoveTrash`
  (params (AmountToRemove :type Integer)))

(event `self.ReceiveTick`
  (params (DeltaSeconds :type "Float (single-precision)"))
  (`TextRenderComponent.K2_SetText` (`self.TextRender`) (`KismetTextLibrary.Conv_IntToText` (`self.CurrentCapacity`)))
  (`SceneComponent.K2_SetWorldRotation` (`self.Arrow`) (`KismetMathLibrary.FindLookAtRotation` (`self.K2_GetActorLocation`) (`SceneComponent.K2_GetComponentLocation` (`Character.Mesh` (`GameplayStatics.GetPlayerCharacter` 0)))) false false))

(fn `UserConstructionScript`)