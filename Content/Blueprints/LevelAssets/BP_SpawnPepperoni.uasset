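; Pepperoni ingredient station that hands BP_Pepperoni items to the player or AI chef, built on a parent with a SpawnIngredient function.
; Interact spawns and attaches pepperoni to an empty-handed player's hold point.
; Collision overlap restocks when the player carries BP_RefillPepperoni, destroying the refill.
; An overlapping empty-handed AI_Chef, when ActiveForAI is set, receives AI-owned pepperoni after a short delay, reducing stock and clearing that flag.
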(event `self.collison.OnComponentBeginOverlap`
  (params (OverlappedComponent :type "PrimitiveComponent Object Reference") (OtherActor :type "Actor Object Reference") (OtherComp :type "PrimitiveComponent Object Reference") (OtherBodyIndex :type Integer) (bFromSweep :type Boolean) (SweepResult :type "HitResult Structure (by ref)"))
  (bind _ai_chef (`self.AI_Chef`))
  (bind _asbp_player_character (cast `/Game/Blueprints/Player/BP_PlayerCharacter` OtherActor)
    (:`then`
      (bind _currentiteminhand (`/Game/Blueprints/Player/BP_PlayerCharacter.CurrentItemInHand` _asbp_player_character))
      (cast `/Game/Blueprints/LevelAssets/BP_RefillPepperoni` _currentiteminhand)
      (`self.AddStock` 10)
      (`self.K2_DestroyActor` _currentiteminhand)
      (set `/Game/Blueprints/Player/BP_PlayerCharacter.CurrentItemInHand` null _asbp_player_character)
      (set `/Game/Blueprints/Player/BP_PlayerCharacter.PlayerHoldingItem?` false _asbp_player_character))
    (:`CastFailed`
      (bind _asai_chef (cast `/Game/Blueprints/AI/AI_Chef/AI_Chef` OtherActor))
      (set `self.AI_Chef` _asai_chef)
      (if (and (`self.ActiveForAI?`) (not (`/Game/Blueprints/AI/AI_Chef/AI_Chef.HoldingItem?` _asai_chef)))
        (`KismetSystemLibrary.Delay` 0.5)
        (bind _returnvalue (`|SpawnActorFromClass` "/Game/Blueprints/LevelAssets/BP_Pepperoni.BP_Pepperoni_C" (`SceneComponent.K2_GetComponentToWorld` (`/Game/Blueprints/AI/AI_Chef/AI_Chef.HoldLocation` (`self.AI_Chef`))) "Undefined" "OverrideRootScale" null null))
        (set `/Game/Blueprints/LevelAssets/BP_Ingredient.AIOwned?` true _returnvalue)
        (`self.K2_AttachToComponent` _returnvalue (`/Game/Blueprints/AI/AI_Chef/AI_Chef.HoldLocation` (`self.AI_Chef`)) "None" "SnapToTarget" "KeepWorld" "KeepWorld" true)
        (set `/Game/Blueprints/AI/AI_Chef/AI_Chef.HoldingItem?` true _ai_chef)
        (bind _output_get (set `/Game/Blueprints/AI/AI_Chef/AI_Chef.CurrentItem` _returnvalue _ai_chef))
        (`self.K2_SetActorRotation` _output_get (struct :`Roll` 90.0) false)
        (`self.ReduceStock` 1)
        (set `self.ActiveForAI?` false)))))

(fn `Interact`
  (params (Interactor :type "/Game/Blueprints/Player/BP_PlayerCharacter Object Reference"))
  (returns (`Success?` :type Boolean))
  (set `self.Player Character REF` Interactor)
  (`self.SpawnIngredient`)
  (return false))

(fn `SpawnIngredient`
  (bind _player_character_ref (`self.Player Character REF`))
  (`parent.SpawnIngredient`)
  (if (not (`/Game/Blueprints/Player/BP_PlayerCharacter.PlayerHoldingItem?` (`self.Player Character REF`)))
    (bind _returnvalue (`|SpawnActorFromClass` "/Game/Blueprints/LevelAssets/BP_Pepperoni.BP_Pepperoni_C" (`SceneComponent.K2_GetComponentToWorld` (`/Game/Blueprints/Player/BP_PlayerCharacter.ItemHoldLocation` (`self.Player Character REF`))) "Undefined" "OverrideRootScale" null null))
    (bind _output_get (set `/Game/Blueprints/Player/BP_PlayerCharacter.CurrentItemInHand` _returnvalue _player_character_ref))
    (`self.K2_AttachToComponent` _output_get (`/Game/Blueprints/Player/BP_PlayerCharacter.ItemHoldLocation` _player_character_ref) "None" "SnapToTarget" "KeepWorld" "KeepWorld" true)
    (set `/Game/Blueprints/Player/BP_PlayerCharacter.PlayerHoldingItem?` true (`self.Player Character REF`))))

(fn `UserConstructionScript`
  (`parent.UserConstructionScript`))