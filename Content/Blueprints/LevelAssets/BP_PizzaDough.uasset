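; Pizza dough actor that players and AI chefs top with cheese, pepperoni or mushrooms, then cook into a pizza.
; Combine events route ingredients by class, destroy each new topping, show its mesh and clear the holder's item.
; Cook starts Tick-driven progress with smoke and a progress bar that a retriggerable delay hides once updates stop.
; Completion swaps the dough for a cooked mesh chosen by cheese and blocks further combining.
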(event `AI_Combine`
  (params (SecondItem :type "/Game/Blueprints/LevelAssets/BP_Ingredient Object Reference") (AI_Chef :type "/Game/Blueprints/AI/AI_Chef/AI_Chef Object Reference"))
  ;[1 1 1] AI Combine
  (set `self.AI Chef REF` AI_Chef)
  (if (not (`self.IsCooked`))
    (`self.Check Ingredient To Combine` SecondItem)
    (set `/Game/Blueprints/AI/AI_Chef/AI_Chef.CurrentItem` null (`self.AI Chef REF`))
    (set `/Game/Blueprints/AI/AI_Chef/AI_Chef.HoldingItem?` false (`self.AI Chef REF`))))

(event `self.Combine`
  (params (SecondItem :type "/Game/Blueprints/LevelAssets/BP_Ingredient Object Reference") (PlayerREF :type "/Game/Blueprints/Player/BP_PlayerCharacter Object Reference"))
  ;[1 1 1] Combine
  (set `self.Player REF` PlayerREF)
  (if (not (`self.IsCooked`))
    (`self.Check Ingredient To Combine` SecondItem)
    (set `/Game/Blueprints/Player/BP_PlayerCharacter.CurrentItemInHand` null (`self.Player REF`))
    (set `/Game/Blueprints/Player/BP_PlayerCharacter.PlayerHoldingItem?` false (`self.Player REF`))))

(event `self.ReceiveTick`
  (params (DeltaSeconds :type "Float (single-precision)"))
  (bind _cookprogress (`self.CookProgress`))
  ;[1 1 1] Cook
  (if (`self.StartCooking?`)
    (`SceneComponent.SetVisibility` (stale `self.Cook` Smoke) true false)
    (set `/Game/Blueprints/LevelAssets/WBP_ProgressBar.Progress` (`self.CookProgress`) (`self.WBP_ProgressBar`))
    (if (< _cookprogress 1.0)
      (set `self.CookProgress` (+ _cookprogress (* DeltaSeconds 0.5)))
      (`SceneComponent.SetVisibility` (`self.ProgressBar`) true false)
      (`KismetSystemLibrary.RetriggerableDelay` 0.15)
      (`SceneComponent.SetVisibility` (`self.ProgressBar`) false false)
      (else
        (`SceneComponent.SetVisibility` (`self.Dough`) false false)
        (if (`self.HasCheese`)
          (`SceneComponent.SetVisibility` (`self.CookedCheese`) true false)
          (else
            (`SceneComponent.SetVisibility` (`self.CookedNone`) true false)))
        (set `self.IsCooked` true)
        (`SceneComponent.SetVisibility` (stale `self.Cook` Smoke) false false)
        (set `self.StartCooking?` false)))))

(event `self.Cook`
  (params (Smoke :type "ParticleSystemComponent Object Reference"))
  ;[1 1 1] Cook
  (set `self.StartCooking?` true))

(fn `Check Ingredient To Combine`
  (params (IngredientToCheck :type "/Game/Blueprints/LevelAssets/BP_Ingredient Object Reference"))
  (locals (SecondIngredient :type "/Game/Blueprints/LevelAssets/BP_Ingredient Object Reference"))
  (bind _output_get (set `local.SecondIngredient` IngredientToCheck))
  (if (== (`GameplayStatics.GetObjectClass` _output_get) "/Game/Blueprints/LevelAssets/BP_Cheese.BP_Cheese_C")
    (`self.CheckIfCheese` (cast `/Game/Blueprints/LevelAssets/BP_Cheese` (`local.SecondIngredient`) :!pure true))
    (elif (== (`GameplayStatics.GetObjectClass` (`local.SecondIngredient`)) "/Game/Blueprints/LevelAssets/BP_PepperoniChopped.BP_PepperoniChopped_C")
      (`self.CheckIfPep` (cast `/Game/Blueprints/LevelAssets/BP_PepperoniChopped` (`local.SecondIngredient`) :!pure true))
      (elif (== (`GameplayStatics.GetObjectClass` (`local.SecondIngredient`)) "/Game/Blueprints/LevelAssets/BP_MushroomChopped.BP_MushroomChopped_C")
        (`self.CheckIfMushroom` (cast `/Game/Blueprints/LevelAssets/BP_MushroomChopped` (`local.SecondIngredient`) :!pure true))))))

(fn `CheckIfCheese`
  (params (CheeseToAdd :type "/Game/Blueprints/LevelAssets/BP_Cheese Object Reference"))
  (if (not (`self.HasCheese`))
    (set `self.HasCheese` true)
    (`self.Combine Ingredient` CheeseToAdd)
    (`SceneComponent.SetVisibility` (`self.CheeseMesh`) true false)))

(fn `CheckIfMushroom`
  (params (MushroomToAdd :type "/Game/Blueprints/LevelAssets/BP_MushroomChopped Object Reference"))
  (if (not (`self.HasMushroom`))
    (set `self.HasMushroom` true)
    (`self.Combine Ingredient` MushroomToAdd)
    (`SceneComponent.SetVisibility` (`self.MushroomsMesh`) true false)))

(fn `CheckIfPep`
  (params (PepperoniToAdd :type "/Game/Blueprints/LevelAssets/BP_PepperoniChopped Object Reference"))
  (if (not (`self.HasPepperoni`))
    (set `self.HasPepperoni` true)
    (`self.Combine Ingredient` PepperoniToAdd)
    (`SceneComponent.SetVisibility` (`self.PepperoniMesh`) true false)))

(fn `Combine Ingredient`
  (params (SecondIngredient :type "/Game/Blueprints/LevelAssets/BP_Ingredient Object Reference"))
  (`self.K2_DetachFromActor` SecondIngredient "KeepWorld" "KeepWorld" "KeepWorld")
  (`self.K2_DestroyActor` SecondIngredient))

(fn `UserConstructionScript`
  (`parent.UserConstructionScript`))