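; BP_CustomerSpawner is a level actor that spawns AI customers while the player has an empty order slot.
; It caches BP_GameplayPC on BeginPlay, then checks its four current order items every Tick for a zero value.
; A Delay on Tick throttles spawning to intervals, placing each AI_Customer randomly inside the SpawnArea box with a waiting-for-order behavior tree and printing a debug message.
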(event `self.ReceiveBeginPlay`
  (bind _asbp_gameplay_pc (cast `/Game/Blueprints/Player/BP_GameplayPC` (`GameplayStatics.GetPlayerController` 0)))
  (set `self.Gameplay_PC_REF` _asbp_gameplay_pc))

(event `self.ReceiveTick`
  (params (DeltaSeconds :type "Float (single-precision)"))
  (bind _gameplay_pc_ref (`self.Gameplay_PC_REF`))
  (bind _spawnarea (`self.SpawnArea`))
  (if (or (== (`/Game/Blueprints/Player/BP_GameplayPC.CurrentOrder1Item` _gameplay_pc_ref) 0) (== (`/Game/Blueprints/Player/BP_GameplayPC.CurrentOrder2Item` _gameplay_pc_ref) 0) (== (`/Game/Blueprints/Player/BP_GameplayPC.CurrentOrder3Item` _gameplay_pc_ref) 0) (== (`/Game/Blueprints/Player/BP_GameplayPC.CurrentOrder4Item` _gameplay_pc_ref) 0))
    (`KismetSystemLibrary.Delay` 5.0)
    (`AIBlueprintHelperLibrary.SpawnAIFromClass` "/Game/Blueprints/AI/AI_Customer/AI_Customer.AI_Customer_C" "/Game/Blueprints/AI/AI_Customer/Customer_WaitingForOrder_BT.Customer_WaitingForOrder_BT" (`KismetMathLibrary.RandomPointInBoundingBox` (`SceneComponent.K2_GetComponentLocation` _spawnarea) (`BoxComponent.GetScaledBoxExtent` _spawnarea)) (struct) false null)
    (`KismetSystemLibrary.PrintString` "CUSTOMER SPAWNED" true true (struct :`R` 0.251974 :`G` 1.0 :`A` 1.0))))

(fn `UserConstructionScript`)