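; BP_StreetLight is a level street light that switches on in the evening based on the in-game hour.
; Every Tick it casts the player character to BP_PlayerCharacter and reads its Hour value.
; Past hour 18 it sets LightOn and raises the SpotLight intensity; otherwise it clears the flag and zeroes the intensity, so it is also dark after midnight.
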(event `self.ReceiveTick`
  (params (DeltaSeconds :type "Float (single-precision)"))
  (bind _asbp_player_character (cast `/Game/Blueprints/Player/BP_PlayerCharacter` (`GameplayStatics.GetPlayerCharacter` 0)))
  (if (> (`/Game/Blueprints/Player/BP_PlayerCharacter.Hour` _asbp_player_character) 18)
    (set `self.LightOn?` true)
    (`LightComponent.SetIntensity` (`self.SpotLight`) 250.0)
    (else
      (set `self.LightOn?` false)
      (`LightComponent.SetIntensity` (`self.SpotLight`) 0.0))))

(fn `UserConstructionScript`)