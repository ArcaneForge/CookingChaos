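; BP_SpawnDough is a dough station that hands pizza dough to AI chefs who overlap its collision component.
; When it is active for AI and the chef's hands are empty, it waits half a second, then spawns BP_PizzaDough at the chef's hold location.
; It attaches the dough there, flags the chef as holding an item, and reduces stock by one.
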(event `self.ReceiveBeginPlay`
  (`parent.ReceiveBeginPlay`))

(event `self.collison.OnComponentBeginOverlap`
  (params (OverlappedComponent :type "PrimitiveComponent Object Reference") (OtherActor :type "Actor Object Reference") (OtherComp :type "PrimitiveComponent Object Reference") (OtherBodyIndex :type Integer) (bFromSweep :type Boolean) (SweepResult :type "HitResult Structure (by ref)"))
  (bind _asai_chef (cast `/Game/Blueprints/AI/AI_Chef/AI_Chef` OtherActor))
  (set `self.AI_Chef` _asai_chef)
  (if (and (`self.ActiveForAI?`) (not (`/Game/Blueprints/AI/AI_Chef/AI_Chef.HoldingItem?` _asai_chef)))
    (`KismetSystemLibrary.Delay` 0.5)
    (bind _returnvalue (`|SpawnActorFromClass` "/Game/Blueprints/LevelAssets/BP_PizzaDough.BP_PizzaDough_C" (`SceneComponent.K2_GetComponentToWorld` (`/Game/Blueprints/AI/AI_Chef/AI_Chef.HoldLocation` (`self.AI_Chef`))) "Undefined" "OverrideRootScale" null null))
    (`self.K2_AttachToComponent` _returnvalue (`/Game/Blueprints/AI/AI_Chef/AI_Chef.HoldLocation` (`self.AI_Chef`)) "None" "SnapToTarget" "KeepWorld" "KeepWorld" true)
    (set `/Game/Blueprints/AI/AI_Chef/AI_Chef.HoldingItem?` true (`self.AI_Chef`))
    (`self.ReduceStock` 1)))

(fn `UserConstructionScript`
  (`parent.UserConstructionScript`))