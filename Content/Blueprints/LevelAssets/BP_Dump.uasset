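; BP_Dump is a trash dump actor that tracks its fill level and shows when it is full.
; A box overlap adds trash when an AI_Binman enters and removes it when an AI_DumpCollector enters.
; Reaching exactly max capacity swaps to the full mesh and shows green smoke, while dropping below max restores the empty mesh and hides the smoke.
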(event `self.AddTrash`
  (params (AmountToAdd :type Integer))
  (bind _output_get (set `self.CurrentCapacity` (+ (`self.CurrentCapacity`) AmountToAdd)))
  (if (== _output_get (`self.MaxCapacity`))
    (`StaticMeshComponent.SetStaticMesh` (`self.StaticMesh`) (`self.FullMesh`))
    (`SceneComponent.SetVisibility` (`self.GreenSmoke`) true false)))

(event `self.RemoveTrash`
  (params (AmountToRemove :type Integer))
  (bind _output_get (set `self.CurrentCapacity` (- (`self.CurrentCapacity`) AmountToRemove)))
  (if (< _output_get (`self.MaxCapacity`))
    (`StaticMeshComponent.SetStaticMesh` (`self.StaticMesh`) (`self.EmptyMesh`))
    (`SceneComponent.SetVisibility` (`self.GreenSmoke`) false false)))

(event `self.ReceiveTick`
  (params (DeltaSeconds :type "Float (single-precision)"))
  (`parent.ReceiveTick` DeltaSeconds))

(event `self.BoxCollision.OnComponentBeginOverlap`
  (params (OverlappedComponent :type "PrimitiveComponent Object Reference") (OtherActor :type "Actor Object Reference") (OtherComp :type "PrimitiveComponent Object Reference") (OtherBodyIndex :type Integer) (bFromSweep :type Boolean) (SweepResult :type "HitResult Structure (by ref)"))
  (cast `/Game/Blueprints/AI/AI_Binman/Binman/AI_Binman` OtherActor
    (:`then`
      (`self.AddTrash` 10))
    (:`CastFailed`
      (cast `/Game/Blueprints/AI/AI_Binman/DumpCollector/AI_DumpCollector` OtherActor)
      (`self.RemoveTrash` 10))))

(fn `UserConstructionScript`
  (`parent.UserConstructionScript`))