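; BP_FireAlarm is a level fire alarm with two point lights that switches between emergency and idle states.
; EmergencyActivated waits briefly, shows both lights and sets a RotatingMovement component spinning.
; EmergencyDeactivate waits the same delay, stops the rotation and hides the lights.
; Both events print a debug message, and nothing inside this Blueprint calls them.
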(event `EmergencyActivated`
  (`KismetSystemLibrary.Delay` 0.2)
  (`SceneComponent.SetVisibility` (`self.PointLight`) true false)
  (`SceneComponent.SetVisibility` (`self.PointLight1`) true false)
  (set `RotatingMovementComponent.RotationRate` (struct :`Roll` 180.0) (`self.RotatingMovement`))
  (`KismetSystemLibrary.PrintString` "EMERGENCY ACTIVATED" true true (struct :`R` 0.146206 :`G` 1.0 :`A` 1.0) 20.0))

(event `EmergencyDeactivate`
  (`KismetSystemLibrary.Delay` 0.2)
  (set `RotatingMovementComponent.RotationRate` (struct) (`self.RotatingMovement`))
  (`SceneComponent.SetVisibility` (`self.PointLight`) false false)
  (`SceneComponent.SetVisibility` (`self.PointLight1`) false false)
  (`KismetSystemLibrary.PrintString` "EMERGENCY DEACTIVATED" true true (struct :`R` 0.146206 :`G` 1.0 :`A` 1.0) 20.0))

(fn `UserConstructionScript`)