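; Tip jar level actor that collects tips from customers and shows growing coin stacks as the total rises.
; When an AI_Customer enters its collision while the jar is active, it adds a small random tip and deactivates itself, with no reactivation in this graph.
; AddTip accumulates the total, then SetCoinStackVisibility reveals up to five coin stack components at rising thresholds, never hiding them again.
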(event `AddTip`
  (params (TipToAdd :type Integer))
  (set `self.CurrentTips` (+ TipToAdd (`self.CurrentTips`)))
  (`self.SetCoinStackVisibility`))

(event `self.Collision.OnComponentBeginOverlap`
  (params (OverlappedComponent :type "PrimitiveComponent Object Reference") (OtherActor :type "Actor Object Reference") (OtherComp :type "PrimitiveComponent Object Reference") (OtherBodyIndex :type Integer) (bFromSweep :type Boolean) (SweepResult :type "HitResult Structure (by ref)"))
  (cast `/Game/Blueprints/AI/AI_Customer/AI_Customer` OtherActor)
  (if (`self.IsActive?`)
    (`self.AddTip` (`KismetMathLibrary.RandomIntegerInRange` 1 10))
    (set `self.IsActive?` false)))

(fn `SetCoinStackVisibility`
  (if (>= (`self.CurrentTips`) 1)
    (`SceneComponent.SetVisibility` (`self.CoinStack1`) true false)
    (if (>= (`self.CurrentTips`) 11)
      (`SceneComponent.SetVisibility` (`self.CoinStack2`) true false)
      (if (>= (`self.CurrentTips`) 21)
        (`SceneComponent.SetVisibility` (`self.CoinStack3`) true false)
        (if (>= (`self.CurrentTips`) 31)
          (`SceneComponent.SetVisibility` (`self.CoinStack4`) true false)
          (if (>= (`self.CurrentTips`) 41)
            (`SceneComponent.SetVisibility` (`self.CoinStack5`) true false)))))))

(fn `UserConstructionScript`)