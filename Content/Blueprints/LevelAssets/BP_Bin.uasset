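; BP_Bin is an interactable rubbish bin that the player fills with held items and an AI binman empties.
; Interact stores the interactor, then destroys its held item and adds one to capacity, or prints a message if the bin is full.
; The BinBag component shows when the count reaches MaxCapacity and hides on removal.
; AI_Binman overlapping BoxCollision empties it only at a hardcoded count of 10, independent of MaxCapacity.
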(event `self.AddTrash`
  (params (AmountToAdd :type Integer))
  (bind _output_get (set `self.CurrentCapacity` (+ (`self.CurrentCapacity`) AmountToAdd)))
  (if (== _output_get (`self.MaxCapacity`))
    (`SceneComponent.SetVisibility` (`self.BinBag`) true false)))

(event `self.RemoveTrash`
  (params (AmountToRemove :type Integer))
  (bind _output_get (set `self.CurrentCapacity` (- (`self.CurrentCapacity`) AmountToRemove)))
  (if (< _output_get (`self.MaxCapacity`))
    (`SceneComponent.SetVisibility` (`self.BinBag`) false false)))

(event `self.ReceiveTick`
  (params (DeltaSeconds :type "Float (single-precision)"))
  (`parent.ReceiveTick` DeltaSeconds))

(event `self.BoxCollision.OnComponentBeginOverlap`
  (params (OverlappedComponent :type "PrimitiveComponent Object Reference") (OtherActor :type "Actor Object Reference") (OtherComp :type "PrimitiveComponent Object Reference") (OtherBodyIndex :type Integer) (bFromSweep :type Boolean) (SweepResult :type "HitResult Structure (by ref)"))
  (cast `/Game/Blueprints/AI/AI_Binman/AI_Binman` OtherActor)
  (if (== (`self.CurrentCapacity`) 10)
    (`self.RemoveTrash` 10)))

(fn `Interact`
  (params (Interactor :type "/Game/Blueprints/Player/BP_PlayerCharacter Object Reference"))
  (returns (`Success?` :type Boolean))
  (set `self.Player Character REF` Interactor)
  (`self.PlayerInteractsWithBin`)
  (return false))

(fn `PlayerInteractsWithBin`
  (bind _player_character_ref (`self.Player Character REF`))
  (if (`/Game/Blueprints/Player/BP_PlayerCharacter.PlayerHoldingItem?` (`self.Player Character REF`))
    (if (< (`self.CurrentCapacity`) (`self.MaxCapacity`))
      (`self.K2_DestroyActor` (`/Game/Blueprints/Player/BP_PlayerCharacter.CurrentItemInHand` (`self.Player Character REF`)))
      (`self.AddTrash` 1)
      (set `/Game/Blueprints/Player/BP_PlayerCharacter.PlayerHoldingItem?` false _player_character_ref)
      (set `/Game/Blueprints/Player/BP_PlayerCharacter.CurrentItemInHand` null _player_character_ref)
      (else
        (`KismetSystemLibrary.PrintString` "BIN FULL")))))

(fn `UserConstructionScript`
  (`parent.UserConstructionScript`))