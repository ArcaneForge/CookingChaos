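; BP_Bat is an interactable bat prop that the player can pick up and put back.
; Interact fakes the transfer by toggling visibility between its own StaticMesh and the player's Bat component, rather than attaching or moving the actor.
; It sets the player's HoldingBat and PlayerHoldingItem flags and starts or stops the bat idle.
; Pickup requires empty hands, and return requires holding the bat.
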(fn `Interact`
  (params (Interactor :type "/Game/Blueprints/Player/BP_PlayerCharacter Object Reference"))
  (returns (`Success?` :type Boolean))
  (bind _playercharacterref (`self.PlayerCharacterREF`))
  (bind _output_get (set `self.PlayerCharacterREF` Interactor))
  (if (`/Game/Blueprints/Player/BP_PlayerCharacter.PlayerHoldingItem?` _output_get)
    (if (`/Game/Blueprints/Player/BP_PlayerCharacter.HoldingBat?` (`self.PlayerCharacterREF`))
      (`SceneComponent.SetVisibility` (`/Game/Blueprints/Player/BP_PlayerCharacter. Bat` _playercharacterref) false false)
      (`TimelineComponent.Stop` (`/Game/Blueprints/Player/BP_PlayerCharacter.ToolIdle` _playercharacterref))
      (set `/Game/Blueprints/Player/BP_PlayerCharacter.HoldingBat?` false (`self.PlayerCharacterREF`))
      (set `/Game/Blueprints/Player/BP_PlayerCharacter.PlayerHoldingItem?` false (`self.PlayerCharacterREF`))
      (`SceneComponent.SetVisibility` (`self.StaticMesh`) true false)
      (return false))
    (else
      (`SceneComponent.SetVisibility` (`/Game/Blueprints/Player/BP_PlayerCharacter. Bat` (`self.PlayerCharacterREF`)) true false)
      (set `/Game/Blueprints/Player/BP_PlayerCharacter.HoldingBat?` true (`self.PlayerCharacterREF`))
      (set `/Game/Blueprints/Player/BP_PlayerCharacter.PlayerHoldingItem?` true (`self.PlayerCharacterREF`))
      (`SceneComponent.SetVisibility` (`self.StaticMesh`) false false)
      (`/Game/Blueprints/Player/BP_PlayerCharacter.BatIdle` (`self.PlayerCharacterREF`))
      (return false))))

(fn `UserConstructionScript`)