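; First-person player character for a pizza kitchen game, handling movement, interaction, chopping, order delivery and the phone menu.
; Interact line-traces forward from the capsule and messages hit actors implementing BPI_Interact.
; Holding Chop opens a Tick gate that chops ingredients on overlapping chopping counters.
; TrySendOrder checks a pizza against the player controller's current orders, then clears the serving counter, completes the order and adds money.
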(event `TrySendOrder`
  (params (PizzaToSend :type "/Game/Blueprints/LevelAssets/BP_PizzaDough Object Reference") (ServingCounter :type "/Game/Blueprints/LevelAssets/BP_ServingCounter Object Reference"))
  ;[1 0.05208 0.05208] Try to complete order - need to change after new interact system
  (bind _asbp_gameplay_pc (cast `/Game/Blueprints/Player/BP_GameplayPC` (`GameplayStatics.GetPlayerController` 0)))
  (`/Game/Blueprints/Player/BP_GameplayPC.GetOrderNumber` _asbp_gameplay_pc PizzaToSend)
  (bind _currentorders (`/Game/Blueprints/Player/BP_GameplayPC.CurrentOrders` _asbp_gameplay_pc))
  (bind _ordertosend (`/Game/Blueprints/Player/BP_GameplayPC.OrderToSend` _asbp_gameplay_pc))
  (if (`KismetArrayLibrary.Array_Contains` _currentorders _ordertosend)
    (`self.K2_DestroyActor` PizzaToSend)
    (set `/Game/Blueprints/LevelAssets/BP_KitchenCounter.ItemOnCounter` null ServingCounter)
    (set `/Game/Blueprints/LevelAssets/BP_KitchenCounter.CounterHasItem?` false ServingCounter)
    (bind _asbp_gameplay_pc_2 (cast `/Game/Blueprints/Player/BP_GameplayPC` (`GameplayStatics.GetPlayerController` 0)))
    (`/Game/Blueprints/Player/BP_GameplayPC.UpdateOrder` _asbp_gameplay_pc_2 (`KismetArrayLibrary.Array_Find` _currentorders _ordertosend) true)
    (setmembers `/Game/Blueprints/Player/BPS_PlayerInfo` :`StructRef` (`self.PlayerInfo`) :`Money` (+ (`.Money_2_129207834C83AA8B34EB46AF5678A6C5` (break `/Game/Blueprints/Player/BPS_PlayerInfo` (`self.PlayerInfo`))) (`.Pizza_2_86EA554143F7D22BFF22A69DADC362CF` (break `/Game/Blueprints/Player/BPS_FoodPrices` (`self.FoodPrices`)))))))

(event `self.ReceiveBeginPlay`
  ;[1 1 1] Set up day/time widget
  (bind _returnvalue (`|CreateWidget` "/Game/Blueprints/UI/MainGame/WBP_Clock.WBP_Clock_C"))
  (`UserWidget.AddToViewport` _returnvalue 0))

(event `InputAxis|Turn`
  (params (AxisValue :type "Float (single-precision)"))
  ;[1 1 1] Character movement
  (`self.AddControllerYawInput` AxisValue))

(event `InputAxis|MoveForward`
  (params (AxisValue :type "Float (single-precision)"))
  ;[1 1 1] Character movement
  (`self.AddMovementInput` (`SceneComponent.GetForwardVector` (`self.FP_Camera`)) AxisValue))

(event `InputAxis|Look Up `
  (params (AxisValue :type "Float (single-precision)"))
  ;[1 1 1] Character movement
  (`self.AddControllerPitchInput` AxisValue))

(event `InputAxis|MoveRight`
  (params (AxisValue :type "Float (single-precision)"))
  ;[1 1 1] Character movement
  (`self.AddMovementInput` (`SceneComponent.GetRightVector` (`self.FP_Camera`)) AxisValue))

(event `InputAction|Interact`
  (params (Key :type "Key Structure"))
  (bind _capsulecomponent (`self.CapsuleComponent`))
  (bind _returnvalue (`SceneComponent.K2_GetComponentLocation` _capsulecomponent))
  ;[1 1 1] Player interacts with actor they are looking at
  (:`Pressed`
    (bind (_outhit _returnvalue_2) (`KismetSystemLibrary.LineTraceSingle` _returnvalue (+ _returnvalue (* (`SceneComponent.GetForwardVector` _capsulecomponent) 150.0)) "TraceTypeQuery1"))
    (if _returnvalue_2
      (bind (_bblockinghit _binitialoverlap _time _distance _location _impactpoint _normal _impactnormal _physmat _hitactor) (`GameplayStatics.BreakHitResult` _outhit))
      (if (`KismetSystemLibrary.DoesImplementInterface` _hitactor "/Game/Blueprints/BPI_Interact.BPI_Interact_C")
        (message `/Game/Blueprints/BPI_Interact.Interact` _hitactor self)))))

(event `self.ReceiveTick`
  (params (DeltaSeconds :type "Float (single-precision)"))
  ;[1 1 1] Chop Ingredient
  (`/Engine/EditorBlueprintResources/StandardMacros.Gate` true :!label _label
    (:`Exit`
      (for _array_element (`self.GetOverlappingActors` "/Script/Engine.Actor")
        (bind _asbp_chopping_counter (cast `/Game/Blueprints/LevelAssets/BP_ChoppingCounter` _array_element))
        (bind _asbp_ingredient (cast `/Game/Blueprints/LevelAssets/BP_Ingredient` (`/Game/Blueprints/LevelAssets/BP_KitchenCounterBase.ItemOnCounter` _asbp_chopping_counter)))
        (if (and (not (`/Game/Blueprints/LevelAssets/BP_Ingredient.IsChopped?` _asbp_ingredient)) (`/Game/Blueprints/LevelAssets/BP_Ingredient.CanBeChopped` _asbp_ingredient))
          (message `/Game/Blueprints/BPI_Chopping.ChopIngredient` _asbp_ingredient DeltaSeconds))))))

(event `InputAction|Chop`
  (params (Key :type "Key Structure"))
  ;[1 1 1] Chop Ingredient
  (:`Pressed`
    (goto _label :!via `Open`))
  (:`Released`
    (goto _label :!via `Close`)))

(fn `BCounterHasItemSet1`
  (params (SpawnTable :type "/Game/Blueprints/LevelAssets/BP_SpawnTable Object Reference"))
  (set `/Game/Blueprints/LevelAssets/BP_KitchenCounter.CounterHasItem?` true SpawnTable))

(fn `InteractWithPhone`
  (bind _returnvalue (`GameplayStatics.GetPlayerController` 0))
  (bind _wbp_phone (`self.WBP_Phone`))
  (`/Engine/EditorBlueprintResources/StandardMacros.IsValid` (`self.WBP_Phone`)
    (:`Is Valid`
      _)
    (:`Is Not Valid`
      (bind _returnvalue_2 (`|CreateWidget` "/Game/Blueprints/UI/MainGame/WBP_PhoneMenu.WBP_PhoneMenu_C"))
      (bind _output_get (set `self.WBP_Phone` _returnvalue_2))
      (`UserWidget.AddToViewport` _output_get 0)))
  (`Widget.SetVisibility` _wbp_phone "Visible")
  (`Widget.SetVisibility` (`/Game/Blueprints/UI/MainGame/WBP_PhoneMenu.PhoneMenu` _wbp_phone) "Visible")
  (`Widget.SetVisibility` (`/Game/Blueprints/UI/MainGame/WBP_PhoneMenu.999Menu` _wbp_phone) "Hidden")
  (`WidgetBlueprintLibrary.SetInputMode_UIOnlyEx` _returnvalue null)
  (set `PlayerController.bShowMouseCursor` true _returnvalue))

(fn `PutDownItemsSetVariables`
  (params (Counter :type "/Game/Blueprints/LevelAssets/BP_KitchenCounter Object Reference"))
  (set `/Game/Blueprints/LevelAssets/BP_KitchenCounter.CounterHasItem?` true Counter)
  (`self.K2_DestroyActor` (`self.CurrentItemInHand`))
  (set `self.CurrentItemInHand` null)
  (set `self.PlayerHoldingItem?` false))

(fn `UserConstructionScript`)