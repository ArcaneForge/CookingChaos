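; Player controller for a pizza order minigame that tracks four timed orders, score and the orders left to complete.
; Tick drains each timer by a fixed per-frame step; UpdateOrder scores successes or timeouts, rerolls that order and shows the end screen at zero orders left.
; RepNotify functions on the order items refresh image, array entry and timer.
; GetOrderNumber maps a cooked pizza's toppings to an order ID.
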(event `self.ReceiveTick`
  (params (DeltaSeconds :type "Float (single-precision)"))
  ;[1 1 1] Start Progress Bar Timers
  (if (`self.StartPBs?`)
    (`|ExecutionSequence`
      (:`then_0`
        (if (> (`self.Order1TimeLeft`) 0.0)
          (set `self.Order1TimeLeft` (- (`self.Order1TimeLeft`) 0.05))
          (else
            (`self.UpdateOrder` 0))))
      (:`then_1`
        (if (> (`self.Order2TimeLeft`) 0.0)
          (set `self.Order2TimeLeft` (- (`self.Order2TimeLeft`) 0.01))
          (else
            (`self.UpdateOrder` 1))))
      (:`then_2`
        (if (> (`self.Order3TimeLeft`) 0.0)
          (set `self.Order3TimeLeft` (- (`self.Order3TimeLeft`) 0.01))
          (else
            (`self.UpdateOrder` 2))))
      (:`then_3`
        (if (> (`self.Order4TimeLeft`) 0.0)
          (set `self.Order4TimeLeft` (- (`self.Order4TimeLeft`) 0.01))
          (else
            (`self.UpdateOrder` 3)))))))

(event `self.ReceiveBeginPlay`
  ;[1 1 1] Set up game - show countdown, orders and progress bars
  (set `self.bShowMouseCursor` false)
  (`self.ShowOrdersWidget`)
  (`self.DisplayWidgets`))

(event `UpdateOrder`
  (params (OrderToUpdate :type Integer) (`OrderSucceeded?` :type Boolean))
  ;[1 1 1] Order Failed/Succeeded - Update Score and generate new order
  (if `OrderSucceeded?`
    (set `self.OrdersLeft` (- (`self.OrdersLeft`) 1))
    (set `self.MinigameScore` (+ (`self.MinigameScore`) 20))
    (else
      (set `self.MinigameScore` (- (`self.MinigameScore`) 20))))
  (switch `int` OrderToUpdate
    (:`0`
      (set `self.CurrentOrder1Item` (`KismetMathLibrary.RandomIntegerInRange` 0 3)))
    (:`1`
      (set `self.CurrentOrder2Item` (`KismetMathLibrary.RandomIntegerInRange` 0 3)))
    (:`2`
      (set `self.CurrentOrder3Item` (`KismetMathLibrary.RandomIntegerInRange` 0 3)))
    (:`3`
      (set `self.CurrentOrder4Item` (`KismetMathLibrary.RandomIntegerInRange` 0 3))))
  (if (== (`self.OrdersLeft`) 0)
    (`self.EndMinigame`)))

(event `EndMinigame`
  ;[1 1 1] End level
  (set `self.bShowMouseCursor` true)
  (`WidgetLayoutLibrary.RemoveAllWidgets`)
  (`self.DisableInput` (`GameplayStatics.GetPlayerCharacter` 0) self)
  (bind _returnvalue (`|CreateWidget` "/Game/Blueprints/UI/MainGame/WBP_LevelEnd.WBP_LevelEnd_C"))
  (bind _output_get (set `self.WBP_MinigameEnd` _returnvalue))
  (`UserWidget.AddToViewport` _output_get 0))

(event `ShowOrdersWidget`
  ;[1 1 1] Set up game - show countdown, orders and progress bars
  (bind _returnvalue (`|CreateWidget` "/Game/Blueprints/UI/MainGame/WBP_Orders.WBP_Orders_C"))
  (`UserWidget.AddToViewport` _returnvalue 0)
  (`self.InitialiseOrderWidget`)
  (set `self.StartPBs?` true))

(event `InitialiseOrderWidget`
  ;[1 1 1] Set up game - show countdown, orders and progress bars
  (bind _output_get (set `self.CurrentOrder1Item` 0))
  (bind _output_get_2 (set `self.CurrentOrder2Item` 1))
  (bind _output_get_3 (set `self.CurrentOrder3Item` 2))
  (bind _output_get_4 (set `self.CurrentOrder4Item` 3))
  (set `self.CurrentOrders` (`|MakeArray` _output_get _output_get_2 _output_get_3 _output_get_4))
  (set `self.OrdersLeft` 3))

(event `GetOrderNumber`
  (params (`Order To Check` :type "/Game/Blueprints/LevelAssets/BP_PizzaDough Object Reference"))
  ;[1 1 1] Get order to send
  (if (`/Game/Blueprints/LevelAssets/BP_PizzaDough.IsCooked` `Order To Check`)
    (if (and (`/Game/Blueprints/LevelAssets/BP_PizzaDough.HasPepperoni` `Order To Check`) (`/Game/Blueprints/LevelAssets/BP_PizzaDough.HasMushroom` `Order To Check`))
      (set `self.OrderToSend` 3)
      (elif (`/Game/Blueprints/LevelAssets/BP_PizzaDough.HasMushroom` `Order To Check`)
        (set `self.OrderToSend` 2)
        (elif (`/Game/Blueprints/LevelAssets/BP_PizzaDough.HasPepperoni` `Order To Check`)
          (set `self.OrderToSend` 1)
          (else
            (set `self.OrderToSend` 0)))))))

(fn `DisplayWidgets`
  (bind _returnvalue (`|CreateWidget` "/Game/Blueprints/UI/MainGame/WBP_Money.WBP_Money_C"))
  (`UserWidget.AddToViewport` _returnvalue 0))

(fn `OnRep_CurrentOrder1Index`
  (set `self.Order1Img` (`|GetArrayItem` (`self.AllOrderImages`) (`self.CurrentOrder1Item`)))
  (`KismetArrayLibrary.Array_Set` (`self.CurrentOrders`) 0 (`self.CurrentOrder1Item`))
  (set `self.Order1TimeLeft` 100.0))

(fn `OnRep_CurrentOrder2Index`
  (set `self.Order2Img` (`|GetArrayItem` (`self.AllOrderImages`) (`self.CurrentOrder2Item`)))
  (`KismetArrayLibrary.Array_Set` (`self.CurrentOrders`) 1 (`self.CurrentOrder2Item`))
  (set `self.Order2TimeLeft` 100.0))

(fn `OnRep_CurrentOrder3Index`
  (set `self.Order3Img` (`|GetArrayItem` (`self.AllOrderImages`) (`self.CurrentOrder3Item`)))
  (`KismetArrayLibrary.Array_Set` (`self.CurrentOrders`) 2 (`self.CurrentOrder3Item`))
  (set `self.Order3TimeLeft` 100.0))

(fn `OnRep_CurrentOrder4Index`
  (set `self.Order4Img` (`|GetArrayItem` (`self.AllOrderImages`) (`self.CurrentOrder4Item`)))
  (`KismetArrayLibrary.Array_Set` (`self.CurrentOrders`) 3 (`self.CurrentOrder4Item`))
  (set `self.Order4TimeLeft` 100.0))

(fn `UserConstructionScript`)