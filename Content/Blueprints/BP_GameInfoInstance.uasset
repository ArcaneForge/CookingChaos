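; BP_GameInfoInstance is a central manager for the game's menu screens and level start.
; Events lazily create and cache the loading screen, main menu and game setup widgets, then add them to the viewport.
; Showing the main menu enables the mouse cursor, while starting the game opens Level1 and hides it.
; Network and travel error-to-string functions return empty strings, and the error display graph is an empty stub.
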(event `ShowLoadingScreen`
  ;[1 1 1] Show loading screen
  (`/Engine/EditorBlueprintResources/StandardMacros.IsValid` (`self.LoadingScreenWidget`)
    (:`Is Valid`
      _)
    (:`Is Not Valid`
      (bind _returnvalue (`|CreateWidget` "/Game/Blueprints/UI/WBP_LoadingScreen.WBP_LoadingScreen_C" (`GameplayStatics.GetPlayerController` 0)))
      (set `self.LoadingScreenWidget` _returnvalue)))
  (`UserWidget.AddToViewport` (`self.LoadingScreenWidget`) 0))

(event `ShowMainMenu`
  (bind _returnvalue (`GameplayStatics.GetPlayerController` 0))
  ;[1 1 1] Create main menu and add to screen (don't recreate it if it already exists) + show mouse cursor
  (`/Engine/EditorBlueprintResources/StandardMacros.IsValid` (`self.MainMenuWidget`)
    (:`Is Valid`
      _)
    (:`Is Not Valid`
      (bind _returnvalue_2 (`|CreateWidget` "/Game/Blueprints/UI/MainMenu/WBP_MainMenu.WBP_MainMenu_C" _returnvalue))
      (set `self.MainMenuWidget` _returnvalue_2)))
  (`UserWidget.AddToViewport` (`self.MainMenuWidget`) 0)
  (set `PlayerController.bShowMouseCursor` true _returnvalue))

(event `StartLevel`
  ;[1 1 1] Start game + hide cursor
  (`GameplayStatics.OpenLevel` "Level1")
  (set `PlayerController.bShowMouseCursor` false (`GameplayStatics.GetPlayerController` 0)))

(event `ShowGameSetupMenu`
  ;[1 1 1] Show game setup menu
  (`/Engine/EditorBlueprintResources/StandardMacros.IsValid` (`self.SetupMenuWidget`)
    (:`Is Valid`
      _)
    (:`Is Not Valid`
      (bind _returnvalue (`|CreateWidget` "/Game/Blueprints/UI/MainMenu/WBP_GameSetupMenu.WBP_GameSetupMenu_C" (`GameplayStatics.GetPlayerController` 0)))
      (set `self.SetupMenuWidget` _returnvalue)))
  (`UserWidget.AddToViewport` (`self.SetupMenuWidget`) 0))

(fn `F Travel Error to String`
  (params (FailureType :type "ETravelFailure Enum" :default "NoLevel"))
  (returns (OutString :type String))
  (return ""))

(fn `F_NetErrorToString`
  (params (FailureType :type "ENetworkFailure Enum" :default "NetDriverAlreadyExists"))
  (returns (OutString :type String))
  (return ""))