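; BP_Moon is a moon actor that fades between day and night states.
; NightTransition plays the DayToNight timeline and DayTransition reverses it.
; The timeline drives moon material opacity, glow density, directional light intensity and an opacity parameter in the FogParams collection (spelled "Opcaity").
; The construction script turns the actor to face Origin and applies a uniform Scale.
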(event `Night Transition`
  (bind (_direction _moon _glow _postprocess _directionallight) (`Timeline|DayToNight` :!label _label)
    (:`Update`
      (`MeshComponent.SetScalarParameterValueOnMaterials` (`self.Moon`) "Opacity" _moon)
      (`MeshComponent.SetScalarParameterValueOnMaterials` (`self.Glow`) "Density" _glow)
      (`LightComponent.SetIntensity` (`self.DirectionalLight`) _directionallight)
      (`KismetMaterialLibrary.SetScalarParameterValue` "/Game/CustomTextures/Materials/FogParams.FogParams" "Opcaity" _postprocess))))

(event `Day Transition`
  (goto _label :!via `Reverse`))

(fn `UserConstructionScript`
  (bind _scale (`self.Scale`))
  (`self.K2_SetActorRotation` (`KismetMathLibrary.Conv_VectorToRotator` (`KismetMathLibrary.Normal` (- (`self.Origin`) (`self.K2_GetActorLocation`)))))
  (`self.SetActorScale3D` (`KismetMathLibrary.MakeVector` _scale _scale _scale)))